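; An early-stage 3D pathfinding actor that so far only builds and visualizes a cubic grid, with no path search yet.
; On BeginPlay it sizes CollisionArray to ArraySize cubed, prints the length, and draws a debug box per cell through nested Z, Y, X loops offset from the root.
; The collision array is never filled, as its write loop is unconnected and Tick is empty.
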(event EventBeginPlay
  (bind _arraysize (Variables|Default|GetArraySize))
  (Utilities|Array|Resize (Variables|Default|GetCollisionArray) (* _arraysize _arraysize _arraysize))
  (Development|PrintString (Utilities|String|ToString(Integer) (Utilities|Array|Length (Variables|Default|GetCollisionArray))) true true "(R=0.000000,G=0.660000,B=1.000000,A=1.000000)" 2e+02)
  ;[1 1 1] z
  (for _index (range 0 (- (Variables|Default|GetArraySize) 1))
    ;[1 1 1] y
    (for _index_2 (range 0 (- (Variables|Default|GetArraySize) 1))
      ;[1 1 1] x
      (for _index_3 (range 0 (- (Variables|Default|GetArraySize) 1))
        (Rendering|Debug|DrawDebugBox (+ (Transformation|GetWorldLocation (Variables|Default|GetDefaultSceneRoot self)) (Math|Vector|MakeVector (* _index_3 (Variables|Default|GetCubeSize)) (* _index_2 (Variables|Default|GetCubeSize)) (* _index (Variables|Default|GetCubeSize)))) (Math|Conversions|ToVector(Float) (- (Variables|Default|GetCubeSize) (Variables|Default|GetMargin))) "(R=0.671748,G=1.000000,B=0.000000,A=1.000000)" "0, 0, 0" 1e+02 2.0)))))

(event Collision|EventActorBeginOverlap
  (params (OtherActor :type Actor%20Object%20Reference)))

(event EventTick
  (params (DeltaSeconds :type Float%20%28single-precision%29)))

(fn ConstructionScript)