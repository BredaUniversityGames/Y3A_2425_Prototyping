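; Smart nav link that makes a Unit crawl across to the link's destination.
; When the smart link is reached, it stores the agent and destination, starts the Unit's crawl and raises a crawling flag.
; While flagged, Tick force-moves that single stored Unit toward the destination.
; A short looping timer, never cleared here, repeatedly lowers the flag and stops the crawl by elapsed time rather than arrival.
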(event Custom|stopCralwing
  (Variables|Default|SetIsCralwing false)
  (Default|Stopcrawling (Variables|Default|GetUnit)))

(event EventBeginPlay)

(event Collision|EventActorBeginOverlap
  (params (OtherActor :type Actor%20Object%20Reference)))

(event EventTick
  (params (DeltaSeconds :type Float%20%28single-precision%29))
  (if (Variables|Default|GetIsCralwing)
    (Default|ForceMoveto (Variables|Default|GetUnit) (Variables|Default|GetDestination) 100)))

(event EventSmartLinkReached
  (params (Agent :type Actor%20Object%20Reference) (Destination :type Vector%20%28by%20ref%29 :default "0, 0, 0"))
  (Variables|Default|SetDestination Destination)
  (bind _asunit (Utilities|Casting|CastToUnit Agent))
  (Variables|Default|SetUnit _asunit)
  (Default|CralwtoDestination _asunit Destination)
  (Variables|Default|SetIsCralwing true)
  (Utilities|Time|SetTimerbyEvent (delegate Custom|stopCralwing) 0.7 true))

(fn ConstructionScript)