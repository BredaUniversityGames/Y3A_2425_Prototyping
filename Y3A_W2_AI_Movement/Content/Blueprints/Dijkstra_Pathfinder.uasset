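; Prototype Dijkstra pathfinder actor that builds and debug-draws a point grid from its location, on construction and at BeginPlay.
; A chain of functions generates the points, sets a clamped test endpoint, then line-traces each point's eight grid neighbours for obstructions.
; Unblocked neighbours are collected as checkable points, with links, boxes and distance values drawn.
; The Dijkstra search itself is a stub: its loop exits immediately without computing a path.
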(event EventBeginPlay
  (CallFunction|RESETDEFAULT)
  (Variables|Default|SetStartPoint (Transformation|GetActorLocation self))
  (Rendering|Debug|FlushPersistentDebugLines)
  (CallFunction|MAINChainAction))

(event Collision|EventActorBeginOverlap
  (params (OtherActor :type Actor%20Object%20Reference)))

(event EventTick
  (params (DeltaSeconds :type Float%20%28single-precision%29)))

(event EventDestroyed
  (Rendering|Debug|FlushPersistentDebugLines))

(fn ConstructionScript
  (Variables|Default|SetStartPoint (Transformation|GetActorLocation self))
  (Rendering|Debug|FlushPersistentDebugLines)
  (CallFunction|MAINChainAction))

(fn MakeArray
  (bind _input (Variables|Default|GetInput))
  (bind _startpoint (Variables|Default|GetStartPoint))
  (for _index (range 0 (- (.size_y (Variables|Default|GetInput)) 1))
    (for _index_2 (range 0 (- (.size_x _input) 1))
      (Utilities|Array|Add (Variables|Default|GetArrayOfPoints) (Math|Vector|MakeVector (+ (* _index_2 (.gap_distance _input)) (.x _startpoint)) (+ (* _index (.gap_distance _input)) (.y _startpoint)) (.z _startpoint)))))
  (CallFunction|SetEndpoint)
  (return))

(fn PrintArray
  (for _array_element (Variables|Default|GetArrayOfPoints)
    (Rendering|Debug|DrawDebugBox _array_element (Math|Conversions|ToVector(Float) (/ (.gap_distance (Variables|Default|GetInput)) 1e+01)) "(R=1.000000,G=0.568227,B=0.009047,A=1.000000)" "0, 0, 0" (Math|Conversions|ToFloat(Integer) (Variables|Default|GetDebugDuration)) 2.0))
  (return))

(fn MAINChainAction
  (CallFunction|MakeArray)
  (CallFunction|AddPointsDataArrayStruct)
  (CallFunction|PrintArray)
  (CallFunction|PrintStartEnd)
  (CallFunction|CheckAllPointsNeighbours)
  (CallFunction|PrintAllValues)
  (CallFunction|DijkstraPathfinding))

(fn SetEndpoint
  (bind (_x_clamped _y_clamped) (CallFunction|ClampXandY (Variables|Default|GetTest%20X) (Variables|Default|GetTest%20Y)))
  (bind _array_index (CallFunction|GetIndexfromXandY _x_clamped _y_clamped))
  (Variables|Default|SetEndPoint (Utilities|Array|Get(acopy) (Variables|Default|GetArrayOfPoints) _array_index)))

(fn PrintStartEnd
  (bind _input (Variables|Default|GetInput))
  (Class|KismetSystemLibrary|DrawDebugConeinDegrees (Variables|Default|GetStartPoint) "0.000000,0.000000,1.000000" (.gap_distance _input) 2e+01 2e+01 5 "(R=0.103765,G=1.000000,B=0.006859,A=1.000000)" (Math|Conversions|ToFloat(Integer) (Variables|Default|GetDebugDuration)) 0.0)
  (Class|KismetSystemLibrary|DrawDebugConeinDegrees (Variables|Default|GetEndPoint) "0.000000,0.000000,1.000000" (.gap_distance _input) 2e+01 2e+01 5 "(R=1.000000,G=0.000000,B=0.027538,A=1.000000)" (Math|Conversions|ToFloat(Integer) (Variables|Default|GetDebugDuration)) 0.0))

(fn GetNeighbourPoints
  (params (ArrayIndex :type Integer))
  (bind _indeciesofneighbours (Variables|Default|GetIndeciesOfNeighbours))
  (Utilities|Array|Clear (Variables|Default|GetIndeciesOfNeighbours))
  (bind (_array_x _array_y) (CallFunction|GetXandYfromIndex ArrayIndex))
  ;[1 1 1] x+1 y-1
  (bind (_x_clamped _y_clamped) (CallFunction|ClampXandY (+ _array_x 1) (- _array_y 1)))
  (bind _array_index (CallFunction|GetIndexfromXandY _x_clamped _y_clamped))
  (Utilities|Array|AddUnique (Variables|Default|GetIndeciesOfNeighbours) _array_index)
  ;[1 1 1] x=0 y-1
  (bind (_x_clamped_2 _y_clamped_2) (CallFunction|ClampXandY _array_x (- _array_y 1)))
  (bind _array_index_2 (CallFunction|GetIndexfromXandY _x_clamped_2 _y_clamped_2))
  (Utilities|Array|AddUnique (Variables|Default|GetIndeciesOfNeighbours) _array_index_2)
  ;[1 1 1] x-1 y-1
  (bind (_x_clamped_3 _y_clamped_3) (CallFunction|ClampXandY (- _array_x 1) (- _array_y 1)))
  (bind _array_index_3 (CallFunction|GetIndexfromXandY _x_clamped_3 _y_clamped_3))
  (Utilities|Array|AddUnique (Variables|Default|GetIndeciesOfNeighbours) _array_index_3)
  ;[1 1 1] x=+1 y=0
  (bind (_x_clamped_4 _y_clamped_4) (CallFunction|ClampXandY (+ _array_x 1) _array_y))
  (bind _array_index_4 (CallFunction|GetIndexfromXandY _x_clamped_4 _y_clamped_4))
  (Utilities|Array|AddUnique (Variables|Default|GetIndeciesOfNeighbours) _array_index_4)
  ;[1 1 1] x-1 y=0
  (bind (_x_clamped_5 _y_clamped_5) (CallFunction|ClampXandY (- _array_x 1) _array_y))
  (bind _array_index_5 (CallFunction|GetIndexfromXandY _x_clamped_5 _y_clamped_5))
  (Utilities|Array|AddUnique (Variables|Default|GetIndeciesOfNeighbours) _array_index_5)
  ;[1 1 1] x=+1 y=+1
  (bind (_x_clamped_6 _y_clamped_6) (CallFunction|ClampXandY (+ _array_x 1) (+ _array_y 1)))
  (bind _array_index_6 (CallFunction|GetIndexfromXandY _x_clamped_6 _y_clamped_6))
  (Utilities|Array|AddUnique (Variables|Default|GetIndeciesOfNeighbours) _array_index_6)
  ;[1 1 1] x=0 y+1
  (bind (_x_clamped_7 _y_clamped_7) (CallFunction|ClampXandY _array_x (+ _array_y 1)))
  (bind _array_index_7 (CallFunction|GetIndexfromXandY _x_clamped_7 _y_clamped_7))
  (Utilities|Array|AddUnique (Variables|Default|GetIndeciesOfNeighbours) _array_index_7)
  ;[1 1 1] x-1 y+1
  (bind (_x_clamped_8 _y_clamped_8) (CallFunction|ClampXandY (- _array_x 1) (+ _array_y 1)))
  (bind _array_index_8 (CallFunction|GetIndexfromXandY _x_clamped_8 _y_clamped_8))
  (Utilities|Array|AddUnique (Variables|Default|GetIndeciesOfNeighbours) _array_index_8)
  (for (_array_element _array_index_9) _indeciesofneighbours
    (if (== _array_element ArrayIndex)
      (Utilities|Array|RemoveIndex _indeciesofneighbours _array_index_9)))
  (return _indeciesofneighbours))

(fn GetXandYfromIndex
  (params (Index :type Integer))
  (bind _startpoint (Variables|Default|GetStartPoint))
  (bind _input (Variables|Default|GetInput))
  (bind _arrayofpoints (Variables|Default|GetArrayOfPoints))
  (bind _output (Utilities|Array|Get(acopy) _arrayofpoints Index))
  (bind _returnvalue (- _output _startpoint))
  (bind _returnvalue_2 (/ _returnvalue (.gap_distance _input)))
  (return (Math|Float|Truncate (.x _returnvalue_2)) (Math|Float|Truncate (.y _returnvalue_2))))

(fn TestNeighbours
  (bind _array_index (CallFunction|GetIndexfromXandY (Variables|Default|GetTest%20X) (Variables|Default|GetTest%20Y)))
  (bind _indeciesofneighbours (CallFunction|GetNeighbourPoints _array_index))
  (Rendering|Debug|DrawDebugSphere (Utilities|Array|Get(acopy) (Variables|Default|GetArrayOfPoints) _array_index) (- (/ (.gap_distance (Variables|Default|GetInput)) 4.0) 1e+01) 12 "(R=0.000000,G=0.097714,B=1.000000,A=1.000000)" (Math|Conversions|ToFloat(Integer) (Variables|Default|GetDebugDuration)) 1.0)
  (for _array_element _indeciesofneighbours
    (Rendering|Debug|DrawDebugSphere (Utilities|Array|Get(acopy) (Variables|Default|GetArrayOfPoints) _array_element) (/ (.gap_distance (Variables|Default|GetInput)) 4.0) 12 "(R=0.982483,G=0.072215,B=1.000000,A=1.000000)" (Math|Conversions|ToFloat(Integer) (Variables|Default|GetDebugDuration)) 1.0)
    (Development|PrintString "BodyLoop"))
  (Development|PrintString "Complete"))

(fn GetIndexfromXandY
  (params (Array%20X :type Integer) (Arra%20Y :type Integer))
  (return (+ (Math|Integer|Clamp(Integer) (+ Array%20X 0) 0 (- (.size_x (Variables|Default|GetInput)) 1)) (* (.size_x (Variables|Default|GetInput)) (Math|Integer|Clamp(Integer) (+ Arra%20Y 0) 0 (- (.size_y (Variables|Default|GetInput)) 1))))))

(fn ClampXandY
  (params (X :type Integer) (Y :type Integer))
  (return (Math|Integer|Clamp(Integer) X 0 (- (.size_x (Variables|Default|GetInput)) 1)) (Math|Integer|Clamp(Integer) Y 0 (- (.size_y (Variables|Default|GetInput)) 1))))

(fn RayCastIndextoIndex
  (params (ArrayIndexStart :type Integer) (ArrayIndexEnd :type Integer) (DebugDraw :type Boolean))
  (bind _arrayofpoints (Variables|Default|GetArrayOfPoints))
  (bind _output (Utilities|Array|Get(acopy) _arrayofpoints ArrayIndexStart))
  (bind _output_2 (Utilities|Array|Get(acopy) _arrayofpoints ArrayIndexEnd))
  (bind _returnvalue (Collision|LineTraceForObjects _output _output_2 (Utilities|Array|MakeArray "ObjectTypeQuery1" "ObjectTypeQuery2" "ObjectTypeQuery4") false 0 "None" true "(R=0.868772,G=1.000000,B=0.000000,A=1.000000)" "(R=1.000000,G=0.019289,B=0.000000,A=1.000000)" 0.0))
  (if _returnvalue
    (if DebugDraw
      (Rendering|Debug|DrawDebugLine _output _output_2 "(R=0.822917,G=0.027724,B=0.000000,A=1.000000)" (Math|Conversions|ToFloat(Integer) (Variables|Default|GetDebugDuration)) 3.0))
    (return false)
    (else
      (if DebugDraw
        (Rendering|Debug|DrawDebugLine _output _output_2 "(R=0.000000,G=0.958333,B=0.170292,A=1.000000)" (Math|Conversions|ToFloat(Integer) (Variables|Default|GetDebugDuration)) 3.0))
      (return true))))

(fn OldTestRayCastSLOW
  (bind _test_x (Variables|Default|GetTest%20X))
  (bind _test_y (Variables|Default|GetTest%20Y))
  (bind _array_index (CallFunction|GetIndexfromXandY (Variables|Default|GetTest%20X) (Variables|Default|GetTest%20Y)))
  (CallFunction|RayCastIndextoIndex _array_index (+ _array_index 1) true)
  (CallFunction|RayCastIndextoIndex _array_index (- _array_index 1) true)
  (bind _array_index_2 (CallFunction|GetIndexfromXandY _test_x (+ _test_y 1)))
  (CallFunction|RayCastIndextoIndex _array_index _array_index_2 true)
  (bind _array_index_3 (CallFunction|GetIndexfromXandY _test_x (- _test_y 1)))
  (CallFunction|RayCastIndextoIndex _array_index _array_index_3 true)
  (bind _array_index_4 (CallFunction|GetIndexfromXandY (+ (Variables|Default|GetTest%20X) 1) (- (Variables|Default|GetTest%20Y) 1)))
  (CallFunction|RayCastIndextoIndex _array_index _array_index_4 true)
  (bind _array_index_5 (CallFunction|GetIndexfromXandY (+ (Variables|Default|GetTest%20X) 1) (+ (Variables|Default|GetTest%20Y) 1)))
  (CallFunction|RayCastIndextoIndex _array_index _array_index_5 true)
  (bind _array_index_6 (CallFunction|GetIndexfromXandY (- (Variables|Default|GetTest%20X) 1) (- (Variables|Default|GetTest%20Y) 1)))
  (CallFunction|RayCastIndextoIndex _array_index _array_index_6 true)
  (bind _array_index_7 (CallFunction|GetIndexfromXandY (- (Variables|Default|GetTest%20X) 1) (+ (Variables|Default|GetTest%20Y) 1)))
  (CallFunction|RayCastIndextoIndex _array_index _array_index_7 true))

(fn DijkstraPathfinding
  (bind _output_get (Variables|Default|SetDijkstraRunning true))
  (Variables|Default|SetCurrentCheckingPoint (Utilities|Array|Get(acopy) (Variables|Default|GetPoints)))
  (while _output_get
    (Variables|Default|SetDijkstraRunning false)))

(fn AddPointsDataArrayStruct
  (Utilities|Array|Clear (Variables|Default|GetPoints))
  (for _array_element (Variables|Default|GetArrayOfPoints)
    (Utilities|Array|Add (Variables|Default|GetPoints) (Utilities|Struct|MakePointParameters false 0 999999.0 _array_element false 0 0)))
  (Utilities|Array|SetArrayElem (Variables|Default|GetPoints) 0 (Utilities|Struct|MakePointParameters false 0 0.0 (Variables|Default|GetStartPoint) false 0 0))
  (return))

(fn SmarterRayCastTest
  (bind _array_index (CallFunction|GetIndexfromXandY (Variables|Default|GetTest%20X) (Variables|Default|GetTest%20Y)))
  (bind _indeciesofneighbours (CallFunction|GetNeighbourPoints _array_index))
  (for _array_element _indeciesofneighbours
    (CallFunction|RayCastIndextoIndex _array_index _array_element true)))

(fn CheckAllPointsNeighbours
  (bind _input (Variables|Default|GetInput))
  (bind _returnvalue (/ (.gap_distance _input) 4.0))
  (for (_array_element _array_index) (Variables|Default|GetPoints)
    (bind _indeciesofneighbours (CallFunction|GetNeighbourPoints _array_index))
    (for _array_element_2 _indeciesofneighbours
      (bind _connects (CallFunction|RayCastIndextoIndex _array_index _array_element_2 true))
      (if _connects
        (Utilities|Array|AddUnique (.connectedtoindecies (Utilities|Array|Get(acopy) (Variables|Default|GetPoints) _array_element_2)) _array_element_2)
        (Rendering|Debug|DrawDebugLine (+ (.position _array_element) (Math|Vector|MakeVector 0.0 0.0 _returnvalue)) (+ (.position (Utilities|Array|Get(acopy) (Variables|Default|GetPoints) _array_element_2)) (Math|Vector|MakeVector 0.0 0.0 _returnvalue)) "(R=0.816609,G=0.822917,B=0.776755,A=1.000000)" (Math|Conversions|ToFloat(Integer) (Variables|Default|GetDebugDuration)) 3.0)
        (Utilities|Array|AddUnique (Variables|Default|GetCheckablePoints) (Utilities|Array|Get(acopy) (Variables|Default|GetPoints) _array_element_2))))
    (Development|PrintString (Utilities|String|ToString(Integer) (Utilities|Array|Length (.connectedtoindecies (Utilities|Array|Get(acopy) (Variables|Default|GetPoints) _array_element_2)))) true true "(R=0.000000,G=0.660000,B=1.000000,A=1.000000)" 1e+01))
  (for _array_element_3 (Variables|Default|GetCheckablePoints)
    (Rendering|Debug|DrawDebugBox :Center (.position _array_element_3) :Extent "10.000000,10.000000,20.000000" :Duration (Math|Conversions|ToFloat(Integer) (Variables|Default|GetDebugDuration)) :Thickness 2.0))
  (return))

(fn PrintAllValues
  (for _array_element (Variables|Default|GetPoints)
    (Rendering|Debug|DrawDebugString (.position _array_element) (Utilities|String|ToString(Float) (.valuefromstart _array_element)) 0 "(R=1.000000,G=0.000000,B=0.876577,A=1.000000)" (Math|Conversions|ToFloat(Integer) (Variables|Default|GetDebugDuration)))))

(fn RESETDEFAULT
  (bind (_input _arrayofpoints _startpoint _endpoint _debugduration _indeciesofneighbours _test_x _test_y _points _testbool _dijkstrarunning _currentcheckingpoint _checkablepoints) (Utilities|GetClassDefaults "Dijkstra_Pathfinder_C"))
  (Variables|Default|SetArrayOfPoints _arrayofpoints)
  (Variables|Default|SetStartPoint _startpoint)
  (Variables|Default|SetEndPoint _endpoint)
  (Variables|Default|SetIndeciesOfNeighbours _indeciesofneighbours)
  (Variables|Default|SetPoints _points)
  (Variables|Default|SetDijkstraRunning _dijkstrarunning)
  (Variables|Default|SetCurrentCheckingPoint _currentcheckingpoint)
  (Variables|Default|SetCheckablePoints _checkablepoints))