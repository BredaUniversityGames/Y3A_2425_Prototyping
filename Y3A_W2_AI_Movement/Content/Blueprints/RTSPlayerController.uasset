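; RTS player controller that lets the player select and command units with the mouse, showing the cursor on begin play.
; Left click traces under the cursor on the Visibility channel and stores a hit PlayerUnit as SelectedUnit, printing debug messages for success or failure.
; Right click orders the valid selected unit to move to the traced impact point through its MoveTo function.
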(event EventBeginPlay
  (Variables|Default|SetbShowMouseCursor true))

(event Input|MouseEvents|LeftMouseButton
  (params (Key :type Key%20Structure :default "None"))
  (:Pressed
    (Development|PrintString "click")
    (bind _asplayer_unit (Utilities|Casting|CastToPlayerUnit (.HitActor (Collision|BreakHitResult (.HitResult (Game|Player|GetHitResultUnderCursorbyChannel "TraceTypeQuery1" true)))))
      (:then
        (Variables|Default|SetSelectedUnit _asplayer_unit)
        (Development|PrintString "Successssss"))
      (:CastFailed
        (Development|PrintString "FAILLEDDD")))))

(event Input|MouseEvents|RightMouseButton
  (params (Key :type Key%20Structure :default "None"))
  (:Pressed
    (Utilities|IsValid (Variables|Default|GetSelectedUnit)
      (:Is%20Valid
        (Default|Moveto (Variables|Default|GetSelectedUnit) (.ImpactPoint (Collision|BreakHitResult (.HitResult (Game|Player|GetHitResultUnderCursorbyChannel "TraceTypeQuery1" true)))))))))

(fn ConstructionScript)